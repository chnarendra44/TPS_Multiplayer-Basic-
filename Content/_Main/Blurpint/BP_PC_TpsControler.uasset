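; Player controller for the third-person shooter prototype that requests a player character when play begins.
; On BeginPlay, only the local controller triggers the spawn request.
; The spawn event hands the controller to GM_TpsPrototype's SpawnPlayer, leaving spawning to the game mode.
; An unconnected leftover chain spawns BP_TpsCharacter at a player start and possesses it, but never runs.
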(event `self.ReceiveBeginPlay`
  (if (`self.IsLocalController`)
    (`self._SpawnCharacter`)))

(event `_SpawnCharacter`
  (bind _asgm_tps_prototype (cast `/Game/_Main/Blurpint/GM_TpsPrototype` (`GameplayStatics.GetGameMode`)))
  (`/Game/_Main/Blurpint/GM_TpsPrototype.SpawnPlayer` _asgm_tps_prototype self))

(fn `UserConstructionScript`)